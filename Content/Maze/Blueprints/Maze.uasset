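; Procedural maze actor that grows endlessly, one row at a time, using Eller's algorithm.
; The construction script builds the initial rows; each MazeTrigger overlap appends another and shifts the trigger forward.
; PrepareRow carries cell sets forward, then MakeRow randomly merges neighbors and places bottom walls, leaving each set an opening.
; Visualize draws walls as mesh instances, re-adding the whole maze on each call without clearing earlier ones.
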(event `self.ReceiveBeginPlay`)

(event `self.MazeTrigger.OnComponentBeginOverlap`
  (params (OverlappedComponent :type "PrimitiveComponent Object Reference") (OtherActor :type "Actor Object Reference") (OtherComp :type "PrimitiveComponent Object Reference") (OtherBodyIndex :type Integer) (bFromSweep :type Boolean) (SweepResult :type "HitResult Structure (by ref)"))
  (`self.AddNewRow` (`|MakeArray`))
  (`self.Visualize`))

(fn `AddNewRow`
  (params (PrevRow :type "Array of /Game/Maze/Blueprints/Cell Structure"))
  (locals (Row :type "Array of /Game/Maze/Blueprints/Cell Structure"))
  (bind _mazetrigger (`self.MazeTrigger`))
  (bind _maze (`self.Maze`))
  (bind _row (`local.Row`))
  (bind _row_2 (`local.Row`))
  (if (> (`KismetArrayLibrary.Array_Length` PrevRow) 0)
    (set `local.Row` PrevRow)
    (else
      (`KismetArrayLibrary.Array_Clear` _row)
      (for _index (range (- (`KismetArrayLibrary.Array_Length` _maze) (`self.Width`)) (+ (`KismetArrayLibrary.Array_LastIndex` _maze) 1))
        (`KismetArrayLibrary.Array_Add` _row (`KismetArrayLibrary.Array_Get` _maze _index)))
      (`KismetSystemLibrary.PrintString` "Last row taken")))
  ;[1 1 1] Prepare Row
  (bind _output_get (set `local.Row` (`self.PrepareRow` (`local.Row`))))
  ;[1 1 1] Fill the row
  (for _array_element _row_2
    (`self.CellPrint` _array_element))
  (bind _resultrow (`self.MakeRow` _row_2))
  ;[1 1 1] Append the Row to the Maze
  (for _array_element_2 _resultrow
    (`KismetArrayLibrary.Array_Add` (`self.Maze`) _array_element_2))
  (`SceneComponent.K2_SetRelativeLocation` _mazetrigger (`KismetMathLibrary.MakeVector` (.x (`SceneComponent.RelativeLocation` _mazetrigger)) (+ (.y (`SceneComponent.RelativeLocation` _mazetrigger)) (`KismetMathLibrary.Conv_IntToDouble` (`self.TileHeight`))) (.z (`SceneComponent.RelativeLocation` _mazetrigger))) false false))

(fn `CellPrint`
  (params (Cell :type "/Game/Maze/Blueprints/Cell Structure"))
  (bind (_index _set _topwall _rightwall _bottomwall _leftwall) (break `/Game/Maze/Blueprints/Cell` Cell))
  (`KismetSystemLibrary.PrintString` (`KismetStringLibrary.Concat_StrStr` "Cell " (`KismetStringLibrary.Conv_IntToString` _index) "in Set: " (`KismetStringLibrary.Conv_IntToString` _set) "walls: " (`KismetStringLibrary.Conv_BoolToString` _topwall) " " (`KismetStringLibrary.Conv_BoolToString` _rightwall) " " (`KismetStringLibrary.Conv_BoolToString` _bottomwall) " " (`KismetStringLibrary.Conv_BoolToString` _leftwall))))

(fn `FindSet`
  (params (set :type Integer) (SetList :type "Array of /Game/Maze/Blueprints/Set Structure"))
  (returns (index :type Integer))
  (locals (FoundIndex :type Integer :default -1))
  (for (_array_element _array_index) SetList
    (if (== set (`.Index_7_16771764AC447934530F7B9FBF2E13A4` (break `/Game/Maze/Blueprints/Set` _array_element)))
      (set `local.FoundIndex` _array_index)
      (break)))
  (return (`local.FoundIndex`)))

(fn `GetCellCoordinates`
  (params (Index :type Integer))
  (returns (X :type "Float (double-precision)") (Y :type "Float (double-precision)"))
  (bind _width (`self.Width`))
  (bind _tile (`self.Tile`))
  (bind (_x _y _x_float _y_float) (`self.IntToGrid` Index _width))
  (return (- (* _tile _x_float) (`KismetMathLibrary.Conv_IntToDouble` (/ (* _width _tile) 2))) (* (`self.TileHeight`) _y_float)))

(fn `MakeBottomWall`
  (params (index :type Integer))
  (bind (_x _y) (`self.GetCellCoordinates` index))
  (`self.MakeWall` (`KismetMathLibrary.MakeTransform` (`KismetMathLibrary.MakeVector` _x (+ _y (`KismetMathLibrary.Conv_IntToDouble` (`self.TileHeight`)))) (struct) (1.0 1.0 1.0))))

(fn `MakeLeftWall`
  (params (index :type Integer))
  (bind (_x _y) (`self.GetCellCoordinates` index))
  (`self.MakeWall` (`KismetMathLibrary.MakeTransform` (`KismetMathLibrary.MakeVector` _x _y) (struct :`Yaw` 90.0) (1.0 1.0 1.0))))

(fn `MakeMaze`
  (params (Width :type Integer))
  (locals (Row :type "Array of /Game/Maze/Blueprints/Cell Structure"))
  (bind _row (`local.Row`))
  (`KismetSystemLibrary.PrintString` "\\n\\n\\n!!!!!! Start to make a Maze !!!!!!!!!!!!")
  (`KismetArrayLibrary.Array_Clear` (`self.Maze`))
  ;[1 1 1] Create the first empty row
  (bind _output_get (set `local.Row` (`|MakeArray`)))
  (for _index (range Width)
    (`KismetArrayLibrary.Array_Add` _output_get (make `/Game/Maze/Blueprints/Cell` :`index` _index :`Set` (+ _index 1) :`TopWall` false)))
  (for _index_2 (range (`self.InitLength`))
    (if (not (== _index_2 0))
      (`KismetArrayLibrary.Array_Clear` _row))
    (`self.AddNewRow` _row))
  (`SceneComponent.K2_SetRelativeLocation` (`self.MazeTrigger`) (`KismetMathLibrary.MakeVector` (.x (`SceneComponent.RelativeLocation` (`self.MazeTrigger`))) (`KismetMathLibrary.Conv_IntToDouble` (`self.TileHeight`)) (.z (`SceneComponent.RelativeLocation` (`self.MazeTrigger`)))) false false))

(fn `MakeRightWall`
  (params (index :type Integer))
  (bind (_x _y) (`self.GetCellCoordinates` index))
  (`self.MakeWall` (`KismetMathLibrary.MakeTransform` (`KismetMathLibrary.MakeVector` (+ _x (`KismetMathLibrary.Conv_IntToDouble` (`self.Tile`))) _y) (struct :`Yaw` 90.0))))

(fn `MakeRow`
  (params (Row :type "Array of /Game/Maze/Blueprints/Cell Structure"))
  (returns (ResultRow :type "Array of /Game/Maze/Blueprints/Cell Structure"))
  (locals (ExistedSets :type "Array of Integer") (NewSet :type Integer :default 1) (NeedJoin :type Integer) (CurrentRow :type "Array of /Game/Maze/Blueprints/Cell Structure") (CurrentSets :type "Array of /Game/Maze/Blueprints/Set Structure") (LeftInSet :type Integer :default 0) (NewRow :type "Array of /Game/Maze/Blueprints/Cell Structure") (SetCells :type "Array of Integer") (FoundSet :type Integer))
  (bind _newrow (`local.NewRow`))
  (bind _leftinset (`local.LeftInSet`))
  (bind _newrow_2 (`local.NewRow`))
  (bind _newrow_3 (`local.NewRow`))
  (bind _newrow_4 (`local.NewRow`))
  (bind _newset (`local.NewSet`))
  (bind _currentrow (`local.CurrentRow`))
  (bind _currentsets (`local.CurrentSets`))
  (bind _currentsets_2 (`local.CurrentSets`))
  (set `local.CurrentRow` Row)
  ;[1 1 1] Collect existing Sets
  (for _array_element (`local.CurrentRow`)
    (bind ((`Set_14_BDB668E58143EACE16863CA738836CFD` _set)) (break `/Game/Maze/Blueprints/Cell` _array_element))
    (if (!= _set 0)
      (`KismetArrayLibrary.Array_AddUnique` (`local.ExistedSets`) _set)))
  ;[1 1 1] Append new cells to Sets
  (for _index (range (+ (`KismetArrayLibrary.Array_LastIndex` _currentrow) 1))
    (bind _item (`KismetArrayLibrary.Array_Get` _currentrow _index))
    (bind ((`Set_14_BDB668E58143EACE16863CA738836CFD` _set_2)) (break `/Game/Maze/Blueprints/Cell` _item))
    (`KismetSystemLibrary.PrintString` (`KismetStringLibrary.Concat_StrStr` "Process cell #" (`KismetStringLibrary.Conv_IntToString` _index) "; with Set #" (`KismetStringLibrary.Conv_IntToString` _set_2)) true true (struct :`R` 0.239645 :`G` 0.36508 :`B` 1.0 :`A` 1.0))
    (bind _returnvalue (`KismetArrayLibrary.Array_Add` _newrow _item))
    (if (== _set_2 0)
      (while (!= (`KismetArrayLibrary.Array_Find` (`local.ExistedSets`) (`local.NewSet`)) -1)
        (`/Engine/EditorBlueprintResources/StandardMacros.IncrementInt` (`local.NewSet`)))
      (bind _structout (setmembers `/Game/Maze/Blueprints/Cell` :`StructRef` (`KismetArrayLibrary.Array_Get` _newrow _returnvalue) :`Set` _newset))
      (`KismetArrayLibrary.Array_Set` _newrow _returnvalue _structout)
      (bind _returnvalue_2 (`KismetArrayLibrary.Array_AddUnique` (`local.ExistedSets`) _newset))
      (`KismetSystemLibrary.PrintString` (`KismetStringLibrary.Concat_StrStr` "Add new Set" (`KismetStringLibrary.Conv_IntToString` _returnvalue_2)))))
  (bind _string (`self.ToString` (`local.ExistedSets`)))
  (`KismetSystemLibrary.PrintString` (`KismetStringLibrary.Concat_StrStr` "Existing sets:" _string))
  ;[1 1 1] Create right walls
  (for (_array_element_2 _array_index) _newrow_2
    (if (== _array_index (`KismetArrayLibrary.Array_LastIndex` _newrow_2))
      ;;[1 1 1] Create right wall for current cell
      (bind _structout_2 (setmembers `/Game/Maze/Blueprints/Cell` :`StructRef` _array_element_2 :`RightWall` true :!label _label))
      (`KismetArrayLibrary.Array_Set` _newrow_2 _array_index _structout_2)
      (else
        (bind (_index_2 _set_3) (break `/Game/Maze/Blueprints/Cell` _array_element_2))
        (bind _returnvalue_3 (+ _array_index 1))
        (bind _item_2 (`KismetArrayLibrary.Array_Get` _newrow_2 _returnvalue_3))
        (if (== _set_3 (`.Set_14_BDB668E58143EACE16863CA738836CFD` (break `/Game/Maze/Blueprints/Cell` _item_2)))
          (goto _label)
          (elif (`KismetMathLibrary.RandomBoolWithWeight` 0.5)
            (goto _label)
            (else
              ;;[1 1 1] Update set for next cell
              (bind _structout_3 (setmembers `/Game/Maze/Blueprints/Cell` :`StructRef` _item_2 :`Set` _set_3 :`RightWall` false))
              (`KismetArrayLibrary.Array_Set` _newrow_2 _returnvalue_3 _structout_3)))))))
  ;[1 1 1] Create Sets array
  (`KismetArrayLibrary.Array_Clear` _currentsets)
  (for _array_element_3 (`local.ExistedSets`)
    (`KismetArrayLibrary.Array_Add` _currentsets (make `/Game/Maze/Blueprints/Set` (`|MakeArray`) _array_element_3)))
  ;[1 1 1] Fill Sets with related Cells
  (for _array_element_4 (`local.NewRow`)
    (bind (_index_3 _set_4) (break `/Game/Maze/Blueprints/Cell` _array_element_4))
    (bind _output_get (set `local.FoundSet` (`self.FindSet` _set_4 _currentsets_2)))
    (bind (_cells _index_4 _hasbottomdoor) (break `/Game/Maze/Blueprints/Set` (`KismetArrayLibrary.Array_Get` _currentsets_2 _output_get)))
    (bind _output_get_2 (set `local.SetCells` _cells))
    (`KismetArrayLibrary.Array_Add` _output_get_2 _index_3)
    (`KismetArrayLibrary.Array_Set` _currentsets_2 _output_get (make `/Game/Maze/Blueprints/Set` _output_get_2 _index_4 _hasbottomdoor)))
  ;[1 1 1] Add bottom walls
  (for (_array_element_5 _array_index_2) (`local.CurrentSets`)
    (bind ((`Cells_4_76C04676B144B03AEAC5FA87CF1C6A88` _cells_2) (`HasBottomDoor_10_7E6BD876DE4B1E74966BCCB14BD70592` _hasbottomdoor_2)) (break `/Game/Maze/Blueprints/Set` _array_element_5))
    (bind _returnvalue_4 (`KismetArrayLibrary.Array_Length` _cells_2))
    (if (!= _returnvalue_4 0)
      (set `local.LeftInSet` _returnvalue_4)
      (for _array_element_6 _cells_2
        (`KismetSystemLibrary.PrintString` (`KismetStringLibrary.Concat_StrStr` "in set left " (`KismetStringLibrary.Conv_IntToString` _leftinset) " cells" "; bottom door: " (`KismetStringLibrary.Conv_BoolToString` _hasbottomdoor_2)))
        (if (and (== _leftinset 1) (not _hasbottomdoor_2))
          (bind _structout_4 (setmembers `/Game/Maze/Blueprints/Set` :`StructRef` _array_element_5 :`HasBottomDoor` true :!label _label_2))
          (`KismetArrayLibrary.Array_Set` (`local.CurrentSets`) _array_index_2 _structout_4)
          (else
            (`KismetSystemLibrary.PrintString` "goto bottom 1")
            (if (`KismetMathLibrary.RandomBoolWithWeight` 0.5)
              (`KismetSystemLibrary.PrintString` "goto bottom 2")
              (bind _structout_5 (setmembers `/Game/Maze/Blueprints/Cell` :`StructRef` (`KismetArrayLibrary.Array_Get` _newrow_3 _array_element_6) :`BottomWall` true))
              (`KismetArrayLibrary.Array_Set` _newrow_3 _array_element_6 _structout_5)
              (else
                (goto _label_2)))))
        (`/Engine/EditorBlueprintResources/StandardMacros.DecrementInt` (`local.LeftInSet`)))
      (else
        (`KismetSystemLibrary.PrintString` "No cells in Set"))))
  ;[1 1 1] Add left wall
  (bind _structout_6 (setmembers `/Game/Maze/Blueprints/Cell` :`StructRef` (`KismetArrayLibrary.Array_Get` _newrow_4) :`LeftWall` true))
  (`KismetArrayLibrary.Array_Set` _newrow_4 0 _structout_6)
  (return _newrow_4))

(fn `MakeTopWall`
  (params (index :type Integer))
  (bind (_x _y) (`self.GetCellCoordinates` index))
  (`self.MakeWall` (`KismetMathLibrary.MakeTransform` (`KismetMathLibrary.MakeVector` _x _y) (struct) (1.0 1.0 1.0))))

(fn `MakeWall`
  (params (Transform :type "Transform Structure"))
  (`InstancedStaticMeshComponent.AddInstance` (`self.Wall`) Transform)
  (return))

(fn `PrepareRow`
  (params (Row :type "Array of /Game/Maze/Blueprints/Cell Structure"))
  (returns (ResultRow :type "Array of /Game/Maze/Blueprints/Cell Structure"))
  (locals (CurrentRow :type "Array of /Game/Maze/Blueprints/Cell Structure"))
  (for _array_element Row
    (bind _structout (setmembers `/Game/Maze/Blueprints/Cell` :`StructRef` _array_element :`RightWall` false))
    ;[1 1 1] Remove from Set
    (if (`.BottomWall_10_3F39A17E7D4763CDB36F65A99A5339E8` (break `/Game/Maze/Blueprints/Cell` _array_element))
      (bind _structout_2 (setmembers `/Game/Maze/Blueprints/Cell` :`StructRef` _structout :`Set` 0))
      (bind _structout_3 (setmembers `/Game/Maze/Blueprints/Cell` :`StructRef` _structout_2 :`BottomWall` false)) ; Clear bottom walls
      (`KismetArrayLibrary.Array_Add` (`local.CurrentRow`) _structout_3)
      (else
        (bind _structout_4 (setmembers `/Game/Maze/Blueprints/Cell` :`StructRef` _structout :`BottomWall` false)) ; Clear bottom walls
        (`KismetArrayLibrary.Array_Add` (`local.CurrentRow`) _structout_4))))
  (return (`local.CurrentRow`)))

(fn `SetsToString`
  (params (sets :type "Array of /Game/Maze/Blueprints/Set Structure"))
  (returns (string :type String))
  (locals (Result :type String :default "Set list: "))
  (for (_array_element _array_index) sets
    (set `local.Result` (`KismetStringLibrary.Concat_StrStr` (`local.Result`) (`KismetStringLibrary.Conv_IntToString` _array_index) ": " (`KismetStringLibrary.Conv_IntToString` (`.Index_7_16771764AC447934530F7B9FBF2E13A4` (break `/Game/Maze/Blueprints/Set` _array_element))) ", ")))
  (return (`local.Result`)))

(fn `ToString`
  (params (array :type "Array of Integer"))
  (returns (string :type String))
  (locals (result :type String))
  (for _array_element array
    (set `local.result` (`KismetStringLibrary.Concat_StrStr` (`local.result`) (`KismetStringLibrary.Conv_IntToString` _array_element) ", ")))
  (return (`local.result`)))

(fn `UserConstructionScript`
  (if (== (`self.TileHeight`) 0)
    (set `self.TileHeight` (`self.Tile`)))
  (`self.MakeMaze` (`self.Width`))
  (`StaticMeshComponent.SetStaticMesh` (`self.Wall`) (`self.WallComponent`))
  (`self.Visualize`))

(fn `Visualize`
  (for (_array_element _array_index) (`self.Maze`)
    (bind (_index _set _topwall _rightwall _bottomwall _leftwall) (break `/Game/Maze/Blueprints/Cell` _array_element))
    (if _topwall
      (`self.MakeTopWall` _array_index))
    (if _rightwall
      (`self.MakeRightWall` _array_index))
    (if _bottomwall
      (`self.MakeBottomWall` _array_index))
    (if _leftwall
      (`self.MakeLeftWall` _array_index))))